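; An actor component that manages health and incoming damage for its owning actor.
; TakeDamage uses the ShouldTakeDamage macro to route each hit to block, normal damage or no damage, based on dead, invincible, blocking and blockable flags.
; Normal damage lowers clamped health, then calls OnDeath or OnDamageResponse.
; Blocked hits leave health untouched but report as damaged with a returned health of zero.
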(event `self.ReceiveBeginPlay`
  (set `self.OwningPlayer` (`self.GetOwner`)))

(fn `Take_Damage`
  (params (damageinfo :type "/Game/DataStructures/Structures/S_DamageInfo Structure"))
  (returns (wasdamaged :type Boolean) (currhealth :type "Float (double-precision)"))
  (locals (currattack :type Text) (availablehit :type Integer))
  (bind (_attackname _damageamount _damagetype _damageresponse _canbeblocked) (break `/Game/DataStructures/Structures/S_DamageInfo` damageinfo))
  (bind _currhealth (`self.currhealth`))
  (`self.ShouldTakeDamage` _canbeblocked
    (:`Blockdamage`
      (return true 0.0))
    (:`Normaldamage`
      (bind _output_get (set `self.currhealth` (`KismetMathLibrary.FClamp` (- _currhealth _damageamount) 0.0 _currhealth)))
      (if (<= _output_get 0.0)
        (set `self.isdead?` true)
        (`self.OnDeath`)
        (else
          (`self.OnDamageResponse`)))
      (return true _output_get))
    (:`Nodamage`
      (return false (`self.currhealth`)))))