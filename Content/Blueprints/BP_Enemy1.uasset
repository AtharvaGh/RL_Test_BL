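; BP_Enemy1 is an enemy Blueprint that exposes health queries and damage intake through its BPCDamageComponent.
; The current health, max health and take-damage functions forward to the component, with take-damage returning whether damage was dealt.
; The dead check is a stub that always returns false, and the event graph and construction script contain no active logic.
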(fn `getcurhealth`
  (returns (Chealth :type "Float (double-precision)"))
  (return (`/Game/Blueprints/BPC_DamageComponent.currhealth` (`self.BPC_DamageComponent`))))

(fn `getmaxhealth`
  (returns (maxhealth :type "Float (double-precision)"))
  (return (`/Game/Blueprints/BPC_DamageComponent.maxhealth` (`self.BPC_DamageComponent`))))

(fn `isdead?`
  (returns (`dead?` :type Boolean))
  (return false))

(fn `takedamage`
  (params (damageinfo :type "/Game/DataStructures/Structures/S_DamageInfo Structure"))
  (returns (`wasdamaged?` :type Boolean))
  (bind _wasdamaged (`/Game/Blueprints/BPC_DamageComponent.Take_Damage` (`self.BPC_DamageComponent`) damageinfo))
  (return _wasdamaged))

(fn `UserConstructionScript`)