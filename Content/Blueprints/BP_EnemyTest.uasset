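; BP_EnemyTest is a melee enemy character that roams, patrols, chases and attacks the player, with a toggleable training-dummy mode.
; BehaviourUnit runs an Initial/Seeking/Pursue state loop with AIMoveTo; pawn sensing or damage triggers pursuit, and distance checks end it.
; Attacks play async-loaded montages with timeline-driven facing, motion warping and sword sphere traces.
; BPCDamageComponent drives hit reactions, brief invincibility, death and a camera-facing health bar.
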(event `self.ReceiveTick`
  (params (DeltaSeconds :type "Float (single-precision)"))
  (bind _healthbar (`self.HealthBar`))
  ;[0.6213 0.8011 1] Rotate healthbar towards player
  (if (`SceneComponent.IsVisible` (`self.HealthBar`))
    (`SceneComponent.K2_SetWorldRotation` _healthbar (`KismetMathLibrary.FindLookAtRotation` (`SceneComponent.K2_GetComponentLocation` _healthbar) (`SceneComponent.K2_GetComponentLocation` (`PlayerCameraManager.TransformComponent` (`GameplayStatics.GetPlayerCameraManager` 0)))) false false)))

(event `self.ReceiveBeginPlay`
  ;[0.3222 1 0.5057] EnemySetup
  (`|ExecutionSequence`
    (:`then_0`
      (bind _aswb_enemy_health (cast `/Game/Blueprints/Widgets/WB_EnemyHealth` (`WidgetComponent.GetWidget` (`self.HealthBar`))))
      (bind _output_get (set `self.Enemyhealth` _aswb_enemy_health))
      (set `/Game/Blueprints/Widgets/WB_EnemyHealth.enemyname` (`self.enemyname`) _output_get)
      (set `/Game/Blueprints/Widgets/WB_EnemyHealth.enemyactor` self _output_get)
      (`SceneComponent.SetVisibility` (`self.HealthBar`) false false))
    (:`then_1`
      (`/Game/Blueprints/Widgets/WB_EnemyHealth.updateenemyhealth` (`self.Enemyhealth`)))
    (:`then_2`
      (set `self.EnemyInitalLoc` (`self.K2_GetActorLocation`))
      (`self.BehaviourUnit`))))

(event `/Game/Interfaces/BPI_damagable.trainingdummy`
  ;[0.4558 1 0.9502] Stop all movement and atatcking capabilities
  (`/Engine/EditorBlueprintResources/StandardMacros.FlipFlop`
    (:`A`
      (set `self.isdummy` true))
    (:`B`
      (set `self.isdummy` false)))
  (`self.BehaviourUnit`))

(event `BehaviourUnit`
  (bind _bpc_damagecomponent (`self.BPC_DamageComponent`))
  (bind _returnvalue (`|EnumEquality` (`self.enemystate`) "NewEnumerator2"))
  ;[0.6572 1 0.434 0.458] This controls all the basic AI of the enemy
  (if (not (`self.isdummy`))
    (`/Engine/EditorBlueprintResources/StandardMacros.IsValid` _bpc_damagecomponent
      (:`Is Valid`
        (if (not (`/Game/Blueprints/BPC_DamageComponent.isdead?` _bpc_damagecomponent))
          (switch `/Game/DataStructures/Enums/Enum_EnemyState` (`self.enemystate`)
            (:`NewEnumerator0`
              ;;[0.6208 0.3014 1] InitialStart
              (`|AIMoveTo` self (`NavigationSystemV1.K2_GetRandomReachablePointInRadius` (`self.K2_GetActorLocation`) (`self.roamRadius`) null null) null
                (:`OnSuccess`
                  (`self.UpdatePatrolPoints`)
                  (`KismetSystemLibrary.Delay` (`KismetMathLibrary.RandomFloatInRange` (`self.minWait`) (`self.maxWait`)))
                  (if _returnvalue
                    (`self.ChasePlayer`)
                    (else
                      (set `self.enemystate` "NewEnumerator1")
                      (`self.BehaviourUnit`))))
                (:`OnFail`
                  (`self.BehaviourUnit`))))
            (:`NewEnumerator1`
              ;;[0.5449 0.3503 1] Go to Patrol Point
              (`|AIMoveTo` self (0.0 0.0 0.0) (`self.patrolPointRef`)
                (:`OnSuccess`
                  (`KismetSystemLibrary.Delay` (`KismetMathLibrary.RandomFloatInRange` (`self.minWait`) (`self.maxWait`)))
                  (if _returnvalue
                    (`self.ChasePlayer`))
                  (set `self.enemystate` "NewEnumerator0")
                  (`self.BehaviourUnit`))
                (:`OnFail`
                  (`self.BehaviourUnit`))))
            (:`NewEnumerator2`
              ;;[1 0.1656 0.2054] Chase and attack Player
              (if (not (`/Game/Blueprints/BPC_DamageComponent.isdead?` (`self.BPC_DamageComponent`))) :!label _label
                (`|AIMoveTo` self (0.0 0.0 0.0) (`self.AttackTarget`) (`self.AttackRadius`)
                  (:`OnSuccess`
                    (`/Engine/EditorBlueprintResources/StandardMacros.DoOnce` false :!label _label_2
                      (:`Completed`
                        (set `self.attackingplayer?` true)
                        (bind _asanim_montage (`/Game/Macros/BPML_Character.Asyncloadanim` (`self.attackmontage`))
                          (:`Out`
                            (`MovementComponent.StopMovementImmediately` (`self.CharacterMovement`))
                            (set `self.upperbody` false)
                            (`|PlayMontage` (`self.Mesh`) _asanim_montage
                              (:`then`
                                (`self.TrackPlayer`))
                              (:`OnCompleted`
                                (`KismetSystemLibrary.Delay` (`KismetMathLibrary.RandomFloatInRange` 0.7 1.5) :!label _label_3)
                                (set `self.attackingplayer?` false)
                                (if (not (`/Game/Blueprints/BPC_DamageComponent.isdead?` (`self.BPC_DamageComponent`)))
                                  (`self.ReleaseAttack`)
                                  (`self.BehaviourUnit`)))
                              (:`OnInterrupted`
                                (goto _label_3))))
                          (:`CastFailed`
                            (`self.BehaviourUnit`))))))
                  (:`OnFail`
                    (`self.BehaviourUnit`))))))
          (else
            (`self.Ondeath`)))))))

(event `OnDamageResponse`
  (bind _returnvalue (`self.K2_GetActorLocation`))
  (bind _healthtimerhandle (`self.HealthTimerhandle`))
  ;[1 0.4683 0.7751] OnEnemyHit
  (`GameplayStatics.PlaySoundAtLocation` "/Engine/VREditor/Sounds/VR_ungrab_Cue.VR_ungrab_Cue" _returnvalue (struct) 1.0 1.0 0.0 null null null null)
  (`NiagaraFunctionLibrary.SpawnSystemAtLocation` "/Game/MixedVFX/Particles/Slashes/SeparateParts/Hits/NS_VampireSlash_Hit.NS_VampireSlash_Hit" _returnvalue)
  (`SceneComponent.SetVisibility` (`self.HealthBar`) true false)
  (if (`KismetSystemLibrary.K2_IsValidTimerHandle` _healthtimerhandle)
    (`KismetSystemLibrary.K2_ClearAndInvalidateTimerHandle` _healthtimerhandle)
    (set `/Game/Blueprints/BPC_DamageComponent.isinvincible` true (`self.BPC_DamageComponent`))
    (bind _returnvalue_2 (`KismetSystemLibrary.K2_SetTimerDelegate` (delegate `Invincibilityframes`) 0.2))
    (set `self.InvincibilityTimerhandle` _returnvalue_2)
    (bind _returnvalue_3 (`KismetSystemLibrary.K2_SetTimerDelegate` (delegate `Removehealthbar`) 3.0))
    (set `self.HealthTimerhandle` _returnvalue_3)
    (if (`SkeletalMeshComponent.IsPlaying` (`self.Mesh`))
      (`self.StopAnimMontage` (`self.ATTMon`)))
    (`MovementComponent.StopMovementImmediately` (`self.CharacterMovement`))
    (set `self.upperbody` true)
    (`|PlayMontage` (`self.Mesh`) "/Game/Animations/StandingReactLargeFromRight_UE_Montage.StandingReactLargeFromRight_UE_Montage" 1.5
      (:`OnCompleted`
        _)
      (:`OnInterrupted`
        _))
    (set `self.upperbody` false)
    (`KismetSystemLibrary.Delay` 1.0)
    (`self.BehaviourUnit`)
    (else
      (set `self.upperbody` true)
      (`|PlayMontage` (`self.Mesh`) "/Game/Animations/StandingReactLargeFromRight_UE_Montage.StandingReactLargeFromRight_UE_Montage" 1.5
        (:`then`
          (`self.StopAnimMontage` "/Game/Animations/NewStableSwordOutwardSlash_UE_Montage.NewStableSwordOutwardSlash_UE_Montage"))
        (:`OnCompleted`
          (set `self.upperbody` false)
          (`KismetSystemLibrary.Delay` 1.0)
          (`self.BehaviourUnit`))))))

(event `Invincibilityframes`
  ;[1 0.4683 0.7751] OnEnemyHit
  (set `/Game/Blueprints/BPC_DamageComponent.isinvincible` false (`self.BPC_DamageComponent`))
  (`KismetSystemLibrary.K2_ClearAndInvalidateTimerHandle` (`self.InvincibilityTimerhandle`)))

(event `Removehealthbar`
  ;[1 0.4683 0.7751] OnEnemyHit
  (`SceneComponent.SetVisibility` (`self.HealthBar`) false false))

(event `ChasePlayer`
  ;[0.6572 1 0.434 0.458] This controls all the basic AI of the enemy
  ;;[1 0.1656 0.2054] Chase and attack Player
  (`/Engine/EditorBlueprintResources/StandardMacros.IsValid` (`self.BPC_DamageComponent`)
    (:`Is Valid`
      (goto _label))))

(event `/Game/Interfaces/BPI_CanAttack.IsAttacking`
  ;[0.6572 1 0.434 0.458] This controls all the basic AI of the enemy
  ;;[1 0.1656 0.2054] Chase and attack Player
  (set `self.attacking` false))

(event `ReleaseAttack`
  ;[0.6572 1 0.434 0.458] This controls all the basic AI of the enemy
  ;;[1 0.1656 0.2054] Chase and attack Player
  (goto _label_2 :!via `Reset`))

(event `Ondeath`
  (bind _returnvalue (`self.K2_GetActorLocation`))
  ;[1 0.4045 0.3047] Death
  (set `self.upperbody` false)
  (if (`/Game/Blueprints/BPC_DamageComponent.isdead?` (`self.BPC_DamageComponent`))
    (set `self.dead?` true)
    (`/Engine/EditorBlueprintResources/StandardMacros.DoOnce` false
      (:`Completed`
        (`GameplayStatics.PlaySoundAtLocation` "/Engine/VREditor/Sounds/VR_ungrab_Cue.VR_ungrab_Cue" _returnvalue (struct) 1.0 1.0 0.0 null null null null)
        (`NiagaraFunctionLibrary.SpawnSystemAtLocation` "/Game/MixedVFX/Particles/Slashes/SeparateParts/Hits/NS_VampireSlash_Hit.NS_VampireSlash_Hit" _returnvalue)
        (bind _notifyname (`|PlayMontage` (`self.Mesh`) "/Game/Animations/Dying_UE_Montage.Dying_UE_Montage")
          (:`OnNotifyBegin`
            (switch `name` _notifyname
              (:`Delete`
                (`self.K2_DestroyActor`)))))))))

(event `/Game/Interfaces/BPI_CanAttack.HitTrace`
  (bind _rpg_sword (`self.Rpg_Sword`))
  ;[1 0.2532 0.5393 0.633] Helper functions for attacks
  ;;[0.3503 0.555 1] Hit Trace for Melee attacks
  (bind _outhit (`KismetSystemLibrary.SphereTraceSingle` (`SceneComponent.GetSocketLocation` _rpg_sword "start") (`SceneComponent.GetSocketLocation` _rpg_sword "end") 15.0 "TraceTypeQuery1" false (`|MakeArray` self :!type "Actor Object Reference")))
  (bind (_bblockinghit _binitialoverlap _time _distance _location _impactpoint _normal _impactnormal _physmat _hitactor) (`GameplayStatics.BreakHitResult` _outhit))
  (if (`KismetSystemLibrary.DoesImplementInterface` _hitactor "/Game/Interfaces/BPI_damagable.BPI_damagable_C")
    (`/Engine/EditorBlueprintResources/StandardMacros.DoOnce` false :!label _label_4
      (:`Completed`
        (message `/Game/Interfaces/BPI_damagable.takedamage` _hitactor (make `/Game/DataStructures/Structures/S_DamageInfo` "EnemyAttack" 20.0) self)))))

(event `MotionWarping`
  ;[1 0.2532 0.5393 0.633] Helper functions for attacks
  ;;[0.94 0.5744 1] MotionWarping
  (bind _attacktarget (`self.AttackTarget`)
    (:`then`
      (`MotionWarpingComponent.AddOrUpdateWarpTarget` (`self.MotionWarpingC`) (make `MotionWarpingTarget` "AttackTarget" (`self.K2_GetActorLocation` _attacktarget) (`self.K2_GetActorRotation`) null "root")))
    (:`else`)))

(event `/Game/Interfaces/BPI_CanAttack.DamageReset`
  ;[1 0.2532 0.5393 0.633] Helper functions for attacks
  ;;[0.3503 0.555 1] Hit Trace for Melee attacks
  (goto _label_4 :!via `Reset`))

(event `self.PawnSensing.OnSeePawn`
  (params (Pawn :type "Pawn Object Reference"))
  ;[1 0.2532 0.5393 0.633] Helper functions for attacks
  ;;[1 0.7883 0.3785] Register player as an attack target
  (`/Engine/EditorBlueprintResources/StandardMacros.IsValid` Pawn
    (:`Is Valid`
      (if (not (`self.dead?`))
        (set `self.AttackTarget` Pawn)
        (set `self.enemystate` "NewEnumerator2" :!label _label_5))
      (`self.BehaviourUnit` :!label _label_6)
      (`self.DisengageAttack`))))

(event `TrackPlayer`
  ;[1 0.2532 0.5393 0.633] Helper functions for attacks
  ;;[0.1851 0.2187 1] Track Player when attacking
  (bind _attacktarget (`self.AttackTarget`)
    (:`then`
      (bind (_direction _turnrate) (`Timeline|FacePlayer` :!via `PlayFromStart`)
        (:`Update`
          (bind (_returnvalue_roll _returnvalue_pitch _returnvalue_yaw) (`KismetMathLibrary.BreakRotator` (`KismetMathLibrary.FindLookAtRotation` (`self.K2_GetActorLocation`) (`self.K2_GetActorLocation` _attacktarget))))
          (`self.K2_SetActorRotation` (`KismetMathLibrary.MakeRotator` 0.0 0.0 (`KismetMathLibrary.Lerp` (.yaw (`self.K2_GetActorRotation`)) _returnvalue_yaw _turnrate))))
        (:`Finished`
          (`KismetSystemLibrary.Delay` 0.2))))
    (:`else`)))

(event `EnemyDamaged`
  (params (Instigator :type "Pawn Object Reference"))
  ;[1 0.2532 0.5393 0.633] Helper functions for attacks
  ;;[1 0.7883 0.3785] Register player as an attack target
  (`/Engine/EditorBlueprintResources/StandardMacros.IsValid` Instigator
    (:`Is Valid`
      (if (not (`self.dead?`))
        (set `self.AttackTarget` Instigator)
        (goto _label_5)
        (else
          (goto _label_6))))))

(event `DisengageAttack`
  ;[1 0.2532 0.5393 0.633] Helper functions for attacks
  ;;[0.34 0.1864 1] StopChasing Player once out of sight
  (bind _attacktarget (`self.AttackTarget`)
    (:`then`
      (if (>= (`self.GetDistanceTo` _attacktarget) (`self.ChaseRange`))
        (set `self.attackingPlayer?` false)
        (set `self.enemystate` "NewEnumerator0")
        (`SceneComponent.SetVisibility` (`self.HealthBar`) false false)
        (`KismetSystemLibrary.Delay` 0.5)
        (`self.BehaviourUnit`)
        (else
          (`KismetSystemLibrary.Delay` 2.0)
          (`self.DisengageAttack`))))
    (:`else`)))

(fn `getcurhealth`
  (returns (Chealth :type "Float (double-precision)"))
  (return (`/Game/Blueprints/BPC_DamageComponent.currhealth` (`self.BPC_DamageComponent`))))

(fn `getmaxhealth`
  (returns (maxhealth :type "Float (double-precision)"))
  (return (`/Game/Blueprints/BPC_DamageComponent.maxhealth` (`self.BPC_DamageComponent`))))

(fn `isdead?`
  (returns (`dead?` :type Boolean))
  (return (`/Game/Blueprints/BPC_DamageComponent.isdead?` (`self.BPC_DamageComponent`))))

(fn `takedamage`
  (params (damageinfo :type "/Game/DataStructures/Structures/S_DamageInfo Structure") (Instigator :type "Pawn Object Reference"))
  (returns (`wasdamaged?` :type Boolean))
  (bind _wasdamaged (`/Game/Blueprints/BPC_DamageComponent.Take_Damage` (`self.BPC_DamageComponent`) damageinfo))
  (if _wasdamaged
    (message `/Game/Interfaces/BPI_enemyhealth.updateenemyhealth` (`self.Enemyhealth`))
    (`self.EnemyDamaged` Instigator)
    (return _wasdamaged)))

(fn `UpdatePatrolPoints`
  (bind _outactors (`GameplayStatics.GetAllActorsOfClass` "/Game/Blueprints/BP_PatrolPoints.BP_PatrolPoints_C"))
  (set `self.patrolPointRef` (`|GetArrayItem` _outactors))
  (for _array_element _outactors
    (if (< (`self.GetDistanceTo` _array_element self) (`self.GetDistanceTo` (`self.patrolPointRef`) self))
      (set `self.patrolPointRef` _array_element))))

(fn `UserConstructionScript`
  (bind _bpc_damagecomponent (`self.BPC_DamageComponent`))
  (`|ExecutionSequence`
    (:`then_0`
      (add `/Game/Blueprints/BPC_DamageComponent.OnDeath` _bpc_damagecomponent (`|CreateDelegate` :!event `Ondeath`))
      (add `/Game/Blueprints/BPC_DamageComponent.OnDamageResponse` _bpc_damagecomponent (`|CreateDelegate` :!event `OnDamageResponse`)))))